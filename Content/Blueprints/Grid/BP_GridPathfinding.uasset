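; BP_GridPathfinding finds a walkable path between two tiles on a grid with six neighbors per tile (hex-style doubled coordinates).
; FindPath runs A* over a cost-sorted discovered list, using a Manhattan-distance heuristic and stopping once the target is discovered.
; Neighbors need a walkable type and a height difference within one tile's Z size.
; GeneratePath walks previous-tile links back from the target, while update and clear callbacks report search data changes.
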(fn `Analyse Next Discovered Tile`
  (returns (`Found Target Tile` :type Boolean))
  (bind _outtilepathdata (`self.PullCheapestTileOutOfDiscoveredList`))
  (set `self.CurrentDiscoveredTile` _outtilepathdata)
  (bind _outneighbors (`self.GetValidTileNeighbors` (`.Index_2_4AA0F759478BC3D865AA19B28B4F7DA8` (break `/Game/Blueprints/Grid/Utilities/STRUCT_PathfidingData` (`self.CurrentDiscoveredTile`)))))
  (set `self.CurrentNeighbors` _outneighbors)
  (while (> (`KismetArrayLibrary.Array_Length` (`self.CurrentNeighbors`)) 0)
    (bind _istargettile (`self.DiscoverNextNeighbor`))
    (if _istargettile
      (return true)))
  (return false))

(fn `ClearGeneratedData`
  (`BlueprintMapLibrary.Map_Clear` (`self.PathfindingData`))
  (`KismetArrayLibrary.Array_Clear` (`self.DiscoveredTileSortingCosts`))
  (`KismetArrayLibrary.Array_Clear` (`self.DiscoveredTileIndexes`))
  (`KismetArrayLibrary.Array_Clear` (`self.AnalysedTileIndexes`))
  (`self.OnPathfindingDataCleared`))

(fn `DiscoverNextNeighbor`
  (returns (IsTargetTile :type Boolean))
  (locals (L_CostFromStart :type Integer) (L_IndexInDiscovered :type Integer :default 0))
  (bind _l_indexindiscovered (`local.L_IndexInDiscovered`))
  (bind (_index _costtoentertile) (break `/Game/Blueprints/Grid/Utilities/STRUCT_PathfidingData` (`self.CurrentNeighbor`)))
  (set `self.CurrentNeighbor` (`|GetArrayItem` (`self.CurrentNeighbors`)))
  (`KismetArrayLibrary.Array_Remove` (`self.CurrentNeighbors`))
  (if (not (`KismetArrayLibrary.Array_Contains` (`self.AnalysedTileIndexes`) (`.Index_2_4AA0F759478BC3D865AA19B28B4F7DA8` (break `/Game/Blueprints/Grid/Utilities/STRUCT_PathfidingData` (`self.CurrentNeighbor`)))))
    (set `local.L_CostFromStart` (+ (`.CostFromStart_8_8767E819427B118CC308BDA9A9B091FA` (break `/Game/Blueprints/Grid/Utilities/STRUCT_PathfidingData` (`self.CurrentDiscoveredTile`))) (`.CostToEnterTile_7_EAEA3E7F454BDC91D9AFC08F11FF6A28` (break `/Game/Blueprints/Grid/Utilities/STRUCT_PathfidingData` (`self.CurrentNeighbor`)))))
    (bind _output_get (set `local.L_IndexInDiscovered` (`KismetArrayLibrary.Array_Find` (`self.DiscoveredTileIndexes`) (`.Index_2_4AA0F759478BC3D865AA19B28B4F7DA8` (break `/Game/Blueprints/Grid/Utilities/STRUCT_PathfidingData` (`self.CurrentNeighbor`))))))
    (if (not (== _output_get -1))
      (bind _output_get_2 (set `self.CurrentNeighbor` (`BlueprintMapLibrary.Map_Find` (`self.PathfindingData`) (`.Index_2_4AA0F759478BC3D865AA19B28B4F7DA8` (break `/Game/Blueprints/Grid/Utilities/STRUCT_PathfidingData` (`self.CurrentNeighbor`))))))
      (if (< (`local.L_CostFromStart`) (`.CostFromStart_8_8767E819427B118CC308BDA9A9B091FA` (break `/Game/Blueprints/Grid/Utilities/STRUCT_PathfidingData` _output_get_2)))
        (`KismetArrayLibrary.Array_Remove` (`self.DiscoveredTileIndexes`) _l_indexindiscovered)
        (`KismetArrayLibrary.Array_Remove` (`self.DiscoveredTileSortingCosts`) _l_indexindiscovered)
        (else
          (return false))))
    (`self.DiscoverTile` (make `/Game/Blueprints/Grid/Utilities/STRUCT_PathfidingData` _index _costtoentertile (`local.L_CostFromStart`) (`self.GetMinCostBetweenTwoTiles` (`.Index_2_4AA0F759478BC3D865AA19B28B4F7DA8` (break `/Game/Blueprints/Grid/Utilities/STRUCT_PathfidingData` (`self.CurrentNeighbor`))) (`self.Target Index`)) (`.Index_2_4AA0F759478BC3D865AA19B28B4F7DA8` (break `/Game/Blueprints/Grid/Utilities/STRUCT_PathfidingData` (`self.CurrentDiscoveredTile`)))))
    (if (`KismetMathLibrary.Equal_IntPointIntPoint` (`.Index_2_4AA0F759478BC3D865AA19B28B4F7DA8` (break `/Game/Blueprints/Grid/Utilities/STRUCT_PathfidingData` (`self.CurrentNeighbor`))) (`self.Target Index`))
      (return true)
      (else
        (return false)))
    (else
      (return false))))

(fn `DiscoverTile`
  (params (InTilePathData :type "/Game/Blueprints/Grid/Utilities/STRUCT_PathfidingData Structure"))
  (bind ((`Index_2_4AA0F759478BC3D865AA19B28B4F7DA8` _index)) (break `/Game/Blueprints/Grid/Utilities/STRUCT_PathfidingData` InTilePathData))
  (`BlueprintMapLibrary.Map_Add` (`self.PathfindingData`) _index InTilePathData)
  (`self.InsertTileInDiscoveredArray` InTilePathData)
  (`self.OnPathfindingDataUpdated` _index))

(fn `FindPath`
  (params (InStart :type "IntPoint Structure") (InTarget :type "IntPoint Structure"))
  (returns (OutPath :type "Array of IntPoint Structure"))
  (set `self.Start Index` InStart)
  (set `self.Target Index` InTarget)
  (`self.ClearGeneratedData`)
  (bind _isvalid (`self.IsInputDataValid`))
  (if _isvalid
    (`self.DiscoverTile` (make `/Game/Blueprints/Grid/Utilities/STRUCT_PathfidingData` (`self.Start Index`) 1 0 (`self.GetMinCostBetweenTwoTiles` (`self.Start Index`) (`self.Target Index`))))
    (while (> (`KismetArrayLibrary.Array_Length` (`self.DiscoveredTileIndexes`)) 0)
      (bind _found_target_tile (`self.Analyse Next Discovered Tile`))
      (if _found_target_tile
        (bind _outpath (`self.GeneratePath`))
        (return _outpath)))
    (return (`|MakeArray` (struct) :!type "IntPoint Structure"))
    (else
      (return (`|MakeArray` (struct) :!type "IntPoint Structure")))))

(fn `GeneratePath`
  (returns (OutPath :type "Array of IntPoint Structure"))
  (locals (L_CurrentIndex :type "IntPoint Structure") (L_InvertedPath :type "Array of IntPoint Structure") (Result :type "Array of IntPoint Structure"))
  (set `local.L_CurrentIndex` (`self.Target Index`))
  (while (!= (`local.L_CurrentIndex`) (`self.Start Index`))
    (`KismetArrayLibrary.Array_Add` (`local.L_InvertedPath`) (`local.L_CurrentIndex`))
    (set `local.L_CurrentIndex` (`.PreviousIndex_13_8B0F65A544B52F5B505C33A3209DE7DA` (break `/Game/Blueprints/Grid/Utilities/STRUCT_PathfidingData` (`BlueprintMapLibrary.Map_Find` (`self.PathfindingData`) (`local.L_CurrentIndex`))))))
  (bind (_arrayindex _arrayelement) (`/Engine/EditorBlueprintResources/StandardMacros.ReverseForEachLoop` (`local.L_InvertedPath`))
    (:`LoopBody`
      (`KismetArrayLibrary.Array_Add` (`local.Result`) _arrayelement))
    (:`Completed`
      (return (`local.Result`)))))

(fn `Get Neighbor Indexes`
  (params (InIndex :type "IntPoint Structure"))
  (returns (OutNeighbors :type "Array of IntPoint Structure"))
  (return (`|MakeArray` (+ (`local.InIndex`) (make `IntPoint` 1 1)) (+ (`local.InIndex`) (make `IntPoint` 0 2)) (+ (`local.InIndex`) (make `IntPoint` -1 1)) (+ (`local.InIndex`) (make `IntPoint` -1 -1)) (+ (`local.InIndex`) (make `IntPoint` 0 -2)) (+ (`local.InIndex`) (make `IntPoint` 1 -1)))))

(fn `GetMinCostBetweenTwoTiles`
  (params (InIndex1 :type "IntPoint Structure") (InIndex2 :type "IntPoint Structure"))
  (returns (OutMinCost :type Integer))
  (bind (_returnvalue_x _returnvalue_y) (break `IntPoint` (- (`local.InIndex1`) (`local.InIndex2`))))
  (return (+ (`KismetMathLibrary.Abs_Int` _returnvalue_x) (`KismetMathLibrary.Abs_Int` _returnvalue_y))))

(fn `GetValidTileNeighbors`
  (params (InIndex :type "IntPoint Structure"))
  (returns (OutNeighbors :type "Array of /Game/Blueprints/Grid/Utilities/STRUCT_PathfidingData Structure"))
  (locals (L_Data :type "/Game/Blueprints/Grid/Utilities/STRUCT_TileData Structure") (L_InData :type "/Game/Blueprints/Grid/Utilities/STRUCT_TileData Structure") (Result :type "Array of /Game/Blueprints/Grid/Utilities/STRUCT_PathfidingData Structure"))
  (bind _l_data_index (break `/Game/Blueprints/Grid/Utilities/STRUCT_TileData` (`local.L_Data`)))
  (bind (_gridtilesize_x _gridtilesize_y _gridtilesize_z) (`KismetMathLibrary.BreakVector` (`/Game/Blueprints/Grid/BP_Grid.GridTileSize` (`self.Grid`))))
  (set `local.L_InData` (`BlueprintMapLibrary.Map_Find` (`/Game/Blueprints/Grid/BP_Grid.GridTiles` (`self.Grid`)) (`local.InIndex`)))
  (bind _outneighbors (`self.Get Neighbor Indexes` (`local.InIndex`)))
  (for _array_element _outneighbors
    (bind _output_get (set `local.L_Data` (`BlueprintMapLibrary.Map_Find` (`/Game/Blueprints/Grid/BP_Grid.GridTiles` (`self.Grid`)) _array_element)))
    (if (`/Game/Blueprints/Grid/Utilities/BFL_TileData.IsTileTypeWalkable` (`.TileType_7_FDFA989E4B40C205CB9B798C73DF83A6` (break `/Game/Blueprints/Grid/Utilities/STRUCT_TileData` _output_get)))
      (if (<= (`KismetMathLibrary.Abs` (- (.z (.location (`.Transform_8_434DC8624A316501811E1AB7C1998F05` (break `/Game/Blueprints/Grid/Utilities/STRUCT_TileData` (`local.L_Data`))))) (.z (.location (`.Transform_8_434DC8624A316501811E1AB7C1998F05` (break `/Game/Blueprints/Grid/Utilities/STRUCT_TileData` (`local.L_InData`))))))) _gridtilesize_z)
        (`KismetArrayLibrary.Array_Add` (`local.Result`) (make `/Game/Blueprints/Grid/Utilities/STRUCT_PathfidingData` _l_data_index 1 999999 999999 (`local.InIndex`))))))
  (return (`local.Result`)))

(fn `InsertTileInDiscoveredArray`
  (params (InTileData :type "/Game/Blueprints/Grid/Utilities/STRUCT_PathfidingData Structure"))
  (locals (L_SortingCost :type Integer))
  (bind ((`CostFromStart_8_8767E819427B118CC308BDA9A9B091FA` _costfromstart) (`MinimumCostToTarget_10_E7E061594EE3542AD9E191B541903CAE` _minimumcosttotarget)) (break `/Game/Blueprints/Grid/Utilities/STRUCT_PathfidingData` InTileData))
  (bind _discoveredtilesortingcosts (`self.DiscoveredTileSortingCosts`))
  (set `local.L_SortingCost` (+ _costfromstart _minimumcosttotarget))
  (if (== (`KismetArrayLibrary.Array_Length` (`self.DiscoveredTileSortingCosts`)) 0)
    (`KismetArrayLibrary.Array_Add` (`self.DiscoveredTileSortingCosts`) (`local.L_SortingCost`) :!label _label)
    (`KismetArrayLibrary.Array_Add` (`self.DiscoveredTileIndexes`) (`.Index_2_4AA0F759478BC3D865AA19B28B4F7DA8` (break `/Game/Blueprints/Grid/Utilities/STRUCT_PathfidingData` (`local.InTileData`))))
    (elif (>= (`local.L_SortingCost`) (`|GetArrayItem` _discoveredtilesortingcosts (`KismetArrayLibrary.Array_LastIndex` _discoveredtilesortingcosts)))
      (goto _label)
      (else
        (for (_array_element _array_index) (`self.DiscoveredTileSortingCosts`)
          (if (>= _array_element (`local.L_SortingCost`))
            (`KismetArrayLibrary.Array_Insert` (`self.DiscoveredTileSortingCosts`) (`local.L_SortingCost`) _array_index)
            (`KismetArrayLibrary.Array_Insert` (`self.DiscoveredTileIndexes`) (`.Index_2_4AA0F759478BC3D865AA19B28B4F7DA8` (break `/Game/Blueprints/Grid/Utilities/STRUCT_PathfidingData` (`local.InTileData`))) _array_index)
            (break)))))))

(fn `IsInputDataValid`
  (returns (IsValid :type Boolean))
  (if (!= (`self.Start Index`) (`self.Target Index`))
    (if (`/Game/Blueprints/Grid/BP_Grid.IsTileWalkable` (`self.Grid`) (`self.Start Index`))
      (if (`/Game/Blueprints/Grid/BP_Grid.IsTileWalkable` (`self.Grid`) (`self.Target Index`))
        (return true)
        (else
          _))))
  (return false))

(fn `PullCheapestTileOutOfDiscoveredList`
  (returns (OutTilePathData :type "/Game/Blueprints/Grid/Utilities/STRUCT_PathfidingData Structure"))
  (locals (L_TileIndex :type "IntPoint Structure"))
  (set `local.L_TileIndex` (`|GetArrayItem` (`self.DiscoveredTileIndexes`)))
  (`KismetArrayLibrary.Array_Remove` (`self.DiscoveredTileSortingCosts`))
  (`KismetArrayLibrary.Array_Remove` (`self.DiscoveredTileIndexes`))
  (`KismetArrayLibrary.Array_Add` (`self.AnalysedTileIndexes`) (`local.L_TileIndex`))
  (return (`BlueprintMapLibrary.Map_Find` (`self.PathfindingData`) (`local.L_TileIndex`))))

(fn `UserConstructionScript`)