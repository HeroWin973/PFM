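; Grid utility actor that draws grid tiles through one InstancedStaticMesh, tinted by tile state.
; Initialization sets mesh, material, base color and collision; tick is disabled.
; InstanceIndexes parallels the instances, mapping grid indices to instance indices so tiles can be replaced, removed or cleared.
; AddInstance writes the highest-priority state color (Selected, Hovered, IsNeighbor, IsInPath) and a filled flag into per-instance custom data for the material.
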(event `self.ReceiveBeginPlay`
  (`self.SetActorTickEnabled` false))

(fn `AddInstance`
  (params (InTransform :type "Transform Structure (by ref)") (InIndex :type "IntPoint Structure (by ref)") (InStates :type "Array of /Game/Blueprints/Grid/Utilities/ENUM_TileState Enum"))
  (locals (L_Index :type Integer :default 0))
  (bind _instancedstaticmesh (`self.InstancedStaticMesh`))
  (bind _l_index (`local.L_Index`))
  (`self.RemoveInstance` InIndex)
  (`InstancedStaticMeshComponent.AddInstance` (`self.InstancedStaticMesh`) (`local.InTransform`) false)
  (bind _returnvalue (`KismetArrayLibrary.Array_Add` (`self.InstanceIndexes`) (`local.InIndex`)))
  (set `local.L_Index` _returnvalue)
  (bind (_outcolor _isfilled) (`self.GetColorFromStates` (`local.InStates`)))
  (bind (_r _g _b) (`KismetMathLibrary.BreakColor` _outcolor))
  (`InstancedStaticMeshComponent.SetCustomDataValue` _instancedstaticmesh _l_index 0 _r false)
  (`InstancedStaticMeshComponent.SetCustomDataValue` _instancedstaticmesh _l_index 1 _g false)
  (`InstancedStaticMeshComponent.SetCustomDataValue` _instancedstaticmesh _l_index 2 _b false)
  (`InstancedStaticMeshComponent.SetCustomDataValue` _instancedstaticmesh _l_index 3 _isfilled false))

(fn `ClearInstances`
  (`InstancedStaticMeshComponent.ClearInstances` (`self.InstancedStaticMesh`))
  (`KismetArrayLibrary.Array_Clear` (`self.InstanceIndexes`)))

(fn `GetColorFromStates`
  (params (InStates :type "Array of /Game/Blueprints/Grid/Utilities/ENUM_TileState Enum"))
  (returns (OutColor :type "LinearColor Structure") (IsFilled :type "Float (double-precision)"))
  (if (== (`KismetArrayLibrary.Array_Length` InStates) 0)
    (return (struct) 0.0)
    (else
      (for _array_element (`|MakeArray` "NewEnumerator2" "NewEnumerator1" "NewEnumerator3" "NewEnumerator4" :!type "/Game/Blueprints/Grid/Utilities/ENUM_TileState Enum")
        (if (`KismetArrayLibrary.Array_Contains` (`local.InStates`) _array_element)
          (return (select `/Game/Blueprints/Grid/Utilities/ENUM_TileState` _array_element :`NewEnumerator1` (struct :`R` 1.0 :`G` 0.830514 :`B` 0.177083 :`A` 1.0) :`NewEnumerator2` (struct :`R` 1.0 :`G` 0.071264 :`A` 1.0) :`NewEnumerator3` (struct :`R` 1.0 :`G` 0.2474 :`B` 0.854077 :`A` 1.0) :`NewEnumerator4` (struct :`R` 0.092316 :`G` 0.71875 :`A` 1.0) :!type "LinearColor Structure") 1.0)))
      (return (struct) 0.0))))

(fn `InitializeGridMeshInst`
  (params (InMesh :type "StaticMesh Object Reference") (InMaterial :type "MaterialInterface Object Reference") (InLinearColor :type "LinearColor Structure") (InCollision :type "ECollisionEnabled Enum" :default "NoCollision"))
  (`|ExecutionSequence`
    (:`then_0`
      (`StaticMeshComponent.SetStaticMesh` (`self.InstancedStaticMesh`) (`local.InMesh`)))
    (:`then_1`
      (`PrimitiveComponent.SetMaterial` (`self.InstancedStaticMesh`) 0 (`local.InMaterial`)))
    (:`then_2`
      (`MeshComponent.SetVectorParameterValueOnMaterials` (`self.InstancedStaticMesh`) "Color" (`KismetMathLibrary.Conv_LinearColorToVector` (`local.InLinearColor`))))
    (:`then_3`
      (`PrimitiveComponent.SetCollisionEnabled` (`self.InstancedStaticMesh`) (`local.InCollision`)))))

(fn `RemoveInstance`
  (params (InIndex :type "IntPoint Structure (by ref)"))
  (if (`KismetArrayLibrary.Array_Contains` (`self.InstanceIndexes`) (`local.InIndex`))
    (`InstancedStaticMeshComponent.RemoveInstance` (`self.InstancedStaticMesh`) (`KismetArrayLibrary.Array_Find` (`self.InstanceIndexes`) (`local.InIndex`)))
    (`KismetArrayLibrary.Array_RemoveItem` (`self.InstanceIndexes`) (`local.InIndex`))))

(fn `UserConstructionScript`)