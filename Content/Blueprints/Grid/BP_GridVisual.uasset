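; Visual layer for a hex grid, drawing walkable tiles through a child BP_GridMeshInstance actor.
; Initialization stores the grid reference, configures that actor with a flat hexagon mesh and material, and positions the visual at the origin, raised by a ground offset.
; Tile updates remove the instance by index and re-add it with transform and states only if walkable.
; Destroying the visual clears all instances, and actor tick is disabled on BeginPlay.
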(event `self.ReceiveBeginPlay`
  (`self.SetActorTickEnabled` false))

(fn `DestroyGridVisual`
  (bind _gridmeshinstance (`self.GridMeshInstance`))
  (`/Engine/EditorBlueprintResources/StandardMacros.IsValid` _gridmeshinstance
    (:`Is Valid`
      (`/Game/Blueprints/Grid/Utilities/BP_GridMeshInstance.ClearInstances` _gridmeshinstance))))

(fn `InitializeGridVisual`
  (params (InGrid :type "/Game/Blueprints/Grid/BP_Grid Object Reference"))
  (set `self.In Grid` InGrid)
  (set `self.GridMeshInstance` (cast `/Game/Blueprints/Grid/Utilities/BP_GridMeshInstance` (`ChildActorComponent.ChildActor` (`self.ChildActor_GridMeshInst`)) :!pure true))
  (`/Game/Blueprints/Grid/Utilities/BP_GridMeshInstance.InitializeGridMeshInst` (`self.GridMeshInstance`) "/Game/Art/Meshes/SM_Grid_HexagonFlat.SM_Grid_HexagonFlat" "/Game/Art/Materials/GridMaterials/MI_Grid_Flat_Hex.MI_Grid_Flat_Hex" (struct :`R` 1.0 :`G` 0.885502 :`A` 1.0) "QueryOnly")
  (`self.K2_SetActorLocation` (0.0 0.0 0.0))
  (`self.SetOffsetFromGround` (`self.OffsetFromGround`)))

(fn `SetOffsetFromGround`
  (params (InOffset :type "Float (double-precision)"))
  (bind (_returnvalue_x _returnvalue_y) (`KismetMathLibrary.BreakVector` (`self.K2_GetActorLocation`)))
  (bind _output_get (set `self.OffsetFromGround` InOffset))
  (`self.K2_SetActorLocation` (`KismetMathLibrary.MakeVector` _returnvalue_x _returnvalue_y _output_get)))

(fn `UpdateTileVisual`
  (params (InTileData :type "/Game/Blueprints/Grid/Utilities/STRUCT_TileData Structure"))
  (bind (_intiledata_index _intiledata_tiletype _intiledata_transform _intiledata_states) (break `/Game/Blueprints/Grid/Utilities/STRUCT_TileData` (`local.InTileData`)))
  (bind (_intiledata_index_2 _intiledata_tiletype_2) (break `/Game/Blueprints/Grid/Utilities/STRUCT_TileData` (`local.InTileData`)))
  (`/Game/Blueprints/Grid/Utilities/BP_GridMeshInstance.RemoveInstance` (`self.GridMeshInstance`) _intiledata_index_2)
  (if (`/Game/Blueprints/Grid/Utilities/BFL_TileData.IsTileTypeWalkable` _intiledata_tiletype_2)
    (`/Game/Blueprints/Grid/Utilities/BP_GridMeshInstance.AddInstance` (`self.GridMeshInstance`) _intiledata_transform _intiledata_index _intiledata_states)))

(fn `UserConstructionScript`)