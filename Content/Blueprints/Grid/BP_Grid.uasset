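; Grid actor that builds a flat hex tile grid around its location in the construction script, sized by tile size and count.
; SpawnGrid clears old instances, takes mesh and material from the Hex row of DT_GridShape, then computes a snapped center and bottom-left corner.
; Tiles are scaled instanced static meshes placed with doubled Y indices, stepping by two with alternating parity per X to form the staggered hex layout.
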(fn `CalculateGridCoordinates`
  (returns (BottomLeft :type "Vector Structure") (Center :type "Vector Structure"))
  (locals (L_Center :type "Vector Structure" :default (0.0 0.0 0.0)))
  (bind _gridtilesize_x (`KismetMathLibrary.BreakVector` (`self.GridTileSize`)))
  (set `local.L_Center` (`/Game/Blueprints/Utilities/BFL_Utilities.SnapVectorToVector` (`self.GridCenterLocation`) (* (`self.GridTileSize`) (1.5 1.0 1.0))))
  (return (- (`local.L_Center`) (+ (`/Game/Blueprints/Utilities/BFL_Utilities.SnapVectorToVector` (* (/ (`self.GridTileCount`) (3.0 2.0)) (`self.GridTileSize`)) (* (`self.GridTileSize`) (1.5 1.0 1.0))) (`KismetMathLibrary.MakeVector` (/ _gridtilesize_x 2.0)))) (`local.L_Center`)))

(fn `DestroyGrid`
  (`InstancedStaticMeshComponent.ClearInstances` (`self.InstancedStaticMesh`)))

(fn `GetTileLocationFromGridIndex`
  (params (GridIndex :type "Vector2D Structure"))
  (returns (TileLocation :type "Vector Structure"))
  (return (+ (`self.GridBottomLeftCornerLocation`) (* (`self.GridTileSize`) (* GridIndex (0.75 0.5))))))

(fn `SpawnGrid`
  (params (CenterLocation :type "Vector Structure") (TileSize :type "Vector Structure") (TileCount :type "Vector2D Structure"))
  (locals (L_XIndex :type Integer) (L_YIndex :type Integer) (L_TileTransform :type "Transform Structure") (L_GridShapeData :type "/Game/Blueprints/Structures/STRUCT_GridShapeData Structure"))
  (bind _instancedstaticmesh (`self.InstancedStaticMesh`))
  (bind (_gridtilecount_x _gridtilecount_y) (`KismetMathLibrary.BreakVector2D` (`self.GridTileCount`)))
  (bind _gridtilecount_x_2 (`KismetMathLibrary.BreakVector2D` (`self.GridTileCount`)))
  (set `self.GridCenterLocation` CenterLocation)
  (set `self.GridTileSize` TileSize)
  (set `self.GridTileCount` (`KismetMathLibrary.ToRounded2D` TileCount))
  (`self.DestroyGrid`)
  (bind _returnvalue (`|GetDataTableRow` "/Game/Data/DT_GridShape.DT_GridShape" "Hex")
    (:`then`
      (bind _output_get (set `local.L_GridShapeData` _returnvalue))
      (bind ((`FlatMesh_11_94E894B24DB07246A7C4F39A021C7049` _flatmesh) (`FlatBorderMaterial_17_BF65FB004B9F93DE3D3773BC163CFDED` _flatbordermaterial)) (break `/Game/Blueprints/Structures/STRUCT_GridShapeData` _output_get))
      (`StaticMeshComponent.SetStaticMesh` _instancedstaticmesh _flatmesh)
      (`PrimitiveComponent.SetMaterial` _instancedstaticmesh 0 _flatbordermaterial)
      (bind (_bottomleft _center) (`self.CalculateGridCoordinates`))
      (set `self.GridBottomLeftCornerLocation` _bottomleft)
      (set `self.GridCenterLocation` _center)
      (for _index (range (+ (`KismetMathLibrary.FTrunc` (- _gridtilecount_x_2 1.0)) 1))
        (set `local.L_XIndex` _index)
        (for _index_2 (range (`KismetMathLibrary.SelectInt` 0 1 (`/Game/Blueprints/Utilities/BFL_Utilities.IsIntEven` (`local.L_XIndex`))) (+ (`KismetMathLibrary.FTrunc` (- (* _gridtilecount_y 2.0) 1.0)) 1))
          (set `local.L_YIndex` _index_2)
          (`|ExecutionSequence`
            (:`then_0`
              (bind _output_get_2 (set `local.L_TileTransform` (`KismetMathLibrary.MakeTransform` (`self.GetTileLocationFromGridIndex` (`KismetMathLibrary.MakeVector2D` (`KismetMathLibrary.Conv_IntToDouble` (`local.L_XIndex`)) (`KismetMathLibrary.Conv_IntToDouble` (`local.L_YIndex`)))) (struct) (/ (`self.GridTileSize`) (`.MeshSize_2_9D5A02EF4137B8D0EF6B7A931EF9BE8E` (break `/Game/Blueprints/Structures/STRUCT_GridShapeData` (`local.L_GridShapeData`)))))))
              (`InstancedStaticMeshComponent.AddInstance` (`self.InstancedStaticMesh`) _output_get_2 true))
            (:`then_1`
              (`/Engine/EditorBlueprintResources/StandardMacros.IncrementInt` _index_2))))))
    (:`RowNotFound`
      (`KismetSystemLibrary.PrintString` "Data row for BP_Grid not found!" true true (struct :`R` 1.0 :`B` 0.094455 :`A` 1.0)))))

(fn `UserConstructionScript`
  (`self.SpawnGrid` (`self.K2_GetActorLocation`) (`self.GridTileSize`) (`self.GridTileCount`)))