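; BP_Pawn is a player-controlled camera pawn with spring-arm zoom, planar movement and stepped yaw rotation.
; Axis inputs update a clamped desired zoom and a desired location along the actor's forward and right vectors, without delta-time scaling.
; Tick eases arm length toward the zoom target but sets location directly, without sweep.
; Rotation actions snap yaw by a fixed angle, leaving the stored RotationDesired unused.
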(event `self.ReceiveBeginPlay`
  (set `self.LocationDesired` (`self.K2_GetActorLocation`))
  (set `self.ZoomDesired` (`SpringArmComponent.TargetArmLength` (`self.SpringArm`)))
  (set `self.RotationDesired` (`self.K2_GetActorRotation`)))

(event `InputAxis|ZoomAxis`
  (params (AxisValue :type "Float (single-precision)"))
  (set `self.ZoomDesired` (`KismetMathLibrary.FClamp` (+ (* AxisValue (`self.ZoomSpeed`)) (`self.ZoomDesired`)) (`self.MinZoom`) (`self.MaxZoom`))))

(event `self.ReceiveTick`
  (params (DeltaSeconds :type "Float (single-precision)"))
  (bind _springarm (`self.SpringArm`))
  (set `SpringArmComponent.TargetArmLength` (`KismetMathLibrary.FInterpTo` (`SpringArmComponent.TargetArmLength` _springarm) (`self.ZoomDesired`) DeltaSeconds (`self.ZoomInterp Speed`)) _springarm)
  (`self.K2_SetActorLocation` (`self.LocationDesired`)))

(event `InputAxis|ForwardAxis`
  (params (AxisValue :type "Float (single-precision)"))
  (set `self.LocationDesired` (+ (`self.LocationDesired`) (* (* AxisValue (`self.MoveSpeed`)) (`self.GetActorForwardVector`)))))

(event `InputAxis|RightAxis`
  (params (AxisValue :type "Float (single-precision)"))
  (set `self.LocationDesired` (+ (`self.LocationDesired`) (* (* AxisValue (`self.MoveSpeed`)) (`self.GetActorRightVector`)))))

(event `InputAction|RotationRIght`
  (params (Key :type "Key Structure"))
  (:`Pressed`
    (`self.K2_SetActorRotation` (`KismetMathLibrary.ComposeRotators` (`self.K2_GetActorRotation`) (`KismetMathLibrary.MakeRotator` 0.0 0.0 (`self.AngleToRotate`))))))

(event `InputAction|RotationLeft`
  (params (Key :type "Key Structure"))
  (:`Pressed`
    (`self.K2_SetActorRotation` (`KismetMathLibrary.ComposeRotators` (`self.K2_GetActorRotation`) (`KismetMathLibrary.MakeRotator` 0.0 0.0 (* (`self.AngleToRotate`) -1.0))))))

(fn `UserConstructionScript`)