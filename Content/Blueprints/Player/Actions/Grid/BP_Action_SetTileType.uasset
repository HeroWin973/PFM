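; BP_Action_SetTileType is a grid player action that changes the tile type of the tile at a given index.
; ExecuteAction checks that the index is valid on the PlayerActions grid, then looks up the existing data in GridTiles.
; It writes the tile back through AddGridTile with the action's TileType, preserving its index, transform and states.
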(fn `ExecuteAction`
  (params (InIndex :type "IntPoint Structure"))
  (locals (L_Data :type "/Game/Blueprints/Grid/Utilities/STRUCT_TileData Structure"))
  (bind (_l_data_index _l_data_tiletype _l_data_transform _l_data_states) (break `/Game/Blueprints/Grid/Utilities/STRUCT_TileData` (`local.L_Data`)))
  (if (`/Game/Blueprints/Grid/BP_Grid.IsIndexVaild` (`/Game/Blueprints/Player/BP_PlayerActions.Grid` (`self.PlayerActions`)) (`local.InIndex`))
    (set `local.L_Data` (`BlueprintMapLibrary.Map_Find` (`/Game/Blueprints/Grid/BP_Grid.GridTiles` (`/Game/Blueprints/Player/BP_PlayerActions.Grid` (`self.PlayerActions`))) (`local.InIndex`)))
    (`/Game/Blueprints/Grid/BP_Grid.AddGridTile` (`/Game/Blueprints/Player/BP_PlayerActions.Grid` (`self.PlayerActions`)) (make `/Game/Blueprints/Grid/Utilities/STRUCT_TileData` _l_data_index (`self.TileType`) _l_data_transform _l_data_states))))

(fn `UserConstructionScript`
  (`parent.UserConstructionScript`))