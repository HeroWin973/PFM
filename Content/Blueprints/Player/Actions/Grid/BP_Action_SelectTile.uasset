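; Player grid action that selects a tile, tracking it in PlayerActions and marking it with a tile state on the grid.
; ExecuteAction clears that state from the previous tile, then either marks the new tile or, if the same tile is passed again, resets the selection to a -999 sentinel index.
; EndPlay runs the action with that sentinel to clear the current selection when the action goes away.
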(event `self.ReceiveEndPlay`
  (params (EndPlayReason :type "EEndPlayReason Enum" :default "Destroyed"))
  (`self.ExecuteAction` (make `IntPoint` -999 -999)))

(fn `ExecuteAction`
  (params (InIndex :type "IntPoint Structure"))
  (bind _playeractions (`self.PlayerActions`))
  (bind _playeractions_2 (`self.PlayerActions`))
  (`/Game/Blueprints/Grid/BP_Grid.RemoveStateFromTile` (`/Game/Blueprints/Player/BP_PlayerActions.Grid` _playeractions) (`/Game/Blueprints/Player/BP_PlayerActions.SelectedTile` _playeractions) "NewEnumerator2")
  (if (!= (`/Game/Blueprints/Player/BP_PlayerActions.SelectedTile` (`self.PlayerActions`)) (`local.InIndex`))
    (set `/Game/Blueprints/Player/BP_PlayerActions.SelectedTile` (`local.InIndex`) (`self.PlayerActions`))
    (`/Game/Blueprints/Grid/BP_Grid.AddStateToTile` (`/Game/Blueprints/Player/BP_PlayerActions.Grid` _playeractions_2) (`/Game/Blueprints/Player/BP_PlayerActions.SelectedTile` _playeractions_2) "NewEnumerator2")
    (else
      (set `/Game/Blueprints/Player/BP_PlayerActions.SelectedTile` (make `IntPoint` -999 -999) (`self.PlayerActions`)))))

(fn `UserConstructionScript`
  (`parent.UserConstructionScript`))