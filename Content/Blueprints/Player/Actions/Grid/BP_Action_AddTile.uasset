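; BP_Action_AddTile is a player grid action that adds a tile at a given grid index where the index is not currently valid.
; ExecuteAction traces for ground at the index's grid location through the Grid referenced by PlayerActions.
; It then calls AddGridTile with a fixed tile type, the traced location and the grid's tile scale.
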(fn `ExecuteAction`
  (params (InIndex :type "IntPoint Structure"))
  (bind _grid (`/Game/Blueprints/Player/BP_PlayerActions.Grid` (`self.PlayerActions`)))
  (if (not (`/Game/Blueprints/Grid/BP_Grid.IsIndexVaild` (`/Game/Blueprints/Player/BP_PlayerActions.Grid` (`self.PlayerActions`)) (`local.InIndex`)))
    (bind _outlocation (`/Game/Blueprints/Grid/BP_Grid.TraceForGround` (`/Game/Blueprints/Player/BP_PlayerActions.Grid` (`self.PlayerActions`)) (`/Game/Blueprints/Grid/BP_Grid.GetTileLocationFromGridIndex` _grid (`local.InIndex`))))
    (`/Game/Blueprints/Grid/BP_Grid.AddGridTile` (`/Game/Blueprints/Player/BP_PlayerActions.Grid` (`self.PlayerActions`)) (make `/Game/Blueprints/Grid/Utilities/STRUCT_TileData` (`local.InIndex`) "NewEnumerator2" (`KismetMathLibrary.MakeTransform` _outlocation (struct) (`/Game/Blueprints/Grid/BP_Grid.GetTileScale` _grid))))))

(fn `UserConstructionScript`
  (`parent.UserConstructionScript`))