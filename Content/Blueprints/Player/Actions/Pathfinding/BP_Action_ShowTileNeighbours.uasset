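; Player action that marks the valid neighbours of a given grid tile, as a visual or debug aid for pathfinding.
; ExecuteAction clears one tile state across the grid, asks GridPathfinding for the tile's valid neighbours, then adds that state to each.
; On EndPlay it runs again with an out-of-range sentinel index, apparently to clear the marks when the action is removed.
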(event `self.ReceiveEndPlay`
  (params (EndPlayReason :type "EEndPlayReason Enum" :default "Destroyed"))
  (`self.ExecuteAction` (make `IntPoint` -999 -999)))

(fn `ExecuteAction`
  (params (InIndex :type "IntPoint Structure"))
  (`/Game/Blueprints/Grid/BP_Grid.ClearStateFromTiles` (`/Game/Blueprints/Player/BP_PlayerActions.Grid` (`self.PlayerActions`)) "NewEnumerator3")
  (bind _outneighbors (`/Game/Blueprints/Grid/BP_GridPathfinding.GetValidTileNeighbors` (`/Game/Blueprints/Grid/BP_Grid.Grid Pathfinding` (`/Game/Blueprints/Player/BP_PlayerActions.Grid` (`self.PlayerActions`))) InIndex))
  (for _array_element _outneighbors
    (`/Game/Blueprints/Grid/BP_Grid.AddStateToTile` (`/Game/Blueprints/Player/BP_PlayerActions.Grid` (`self.PlayerActions`)) (break `/Game/Blueprints/Grid/Utilities/STRUCT_PathfidingData` _array_element) "NewEnumerator3")))

(fn `UserConstructionScript`
  (`parent.UserConstructionScript`))