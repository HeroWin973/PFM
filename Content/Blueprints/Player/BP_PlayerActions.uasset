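; BP_PlayerActions handles mouse interaction with the BP_Grid, tracking the hovered tile and running the selected action for left or right click.
; Each tick it updates the tile under the cursor, moving a hover state and raising a change event that repeats held-button actions for drag use.
; SetSelectedActions spawns action actors per button, destroying the old ones, then broadcasts the new selection.
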(event `self.ReceiveBeginPlay`
  (bind _returnvalue (`GameplayStatics.GetPlayerController` 0))
  (bind _returnvalue_2 (`GameplayStatics.GetActorOfClass` "/Game/Blueprints/Grid/BP_Grid.BP_Grid_C"))
  (set `self.Grid` _returnvalue_2)
  (`self.EnableInput` _returnvalue)
  (set `PlayerController.bShowMouseCursor` true _returnvalue))

(event `self.ReceiveTick`
  (params (DeltaSeconds :type "Float (single-precision)"))
  (`self.UpdateHoveredTile`))

(event `Key|LeftMouseButton`
  (params (Key :type "Key Structure"))
  (:`Pressed`
    (`self.UpdateHoveredTile`)
    (set `self.IsLeftClickDown` true)
    (`/Engine/EditorBlueprintResources/StandardMacros.IsValid` (`self.SelectedAction_LeftClick`) :!label _label
      (:`Is Valid`
        (`/Game/Blueprints/Player/Actions/BP_Action.ExecuteAction` (`self.SelectedAction_LeftClick`) (`self.HoveredTile`)))))
  (:`Released`
    (set `self.IsLeftClickDown` false)))

(event `OnHoverTileChanged`
  (`|ExecutionSequence`
    (:`then_0`
      (if (`self.IsLeftClickDown`)
        (goto _label)))
    (:`then_1`
      (if (`self.IsRightClickDown`)
        (`/Engine/EditorBlueprintResources/StandardMacros.IsValid` (`self.SelectedAction_RightClick`) :!label _label_2
          (:`Is Valid`
            (`/Game/Blueprints/Player/Actions/BP_Action.ExecuteAction` (`self.SelectedAction_RightClick`) (`self.HoveredTile`))))))))

(event `Key|RightMouseButton`
  (params (Key :type "Key Structure"))
  (:`Pressed`
    (`self.UpdateHoveredTile`)
    (set `self.IsRightClickDown` true)
    (goto _label_2))
  (:`Released`
    (set `self.IsRightClickDown` false)))

(fn `SetSelectedActions`
  (params (InLeftAction :type "/Game/Blueprints/Player/Actions/BP_Action Class Reference") (InRightAction :type "/Game/Blueprints/Player/Actions/BP_Action Class Reference"))
  (bind _selectedaction_rightclick (`self.SelectedAction_RightClick`))
  (bind _selectedaction_leftclick (`self.SelectedAction_LeftClick`))
  (`|ExecutionSequence`
    (:`then_0`
      (`/Engine/EditorBlueprintResources/StandardMacros.IsValid` _selectedaction_leftclick
        (:`Is Valid`
          (`self.K2_DestroyActor` _selectedaction_leftclick)
          (set `self.SelectedAction_LeftClick` null))
        (:`Is Not Valid`
          _))
      (if (`KismetSystemLibrary.IsValidClass` (`local.InLeftAction`))
        (bind _returnvalue (`|SpawnActorFromClass` (`local.InLeftAction`) (`KismetMathLibrary.MakeTransform` (0.0 0.0 0.0)) "AlwaysSpawn" "MultiplyWithRoot" null self null))
        (set `self.SelectedAction_LeftClick` _returnvalue)))
    (:`then_1`
      (`/Engine/EditorBlueprintResources/StandardMacros.IsValid` _selectedaction_rightclick
        (:`Is Valid`
          (`self.K2_DestroyActor` _selectedaction_rightclick)
          (set `self.SelectedAction_RightClick` null))
        (:`Is Not Valid`
          _))
      (if (`KismetSystemLibrary.IsValidClass` (`local.InRightAction`))
        (bind _returnvalue_2 (`|SpawnActorFromClass` (`local.InRightAction`) (`KismetMathLibrary.MakeTransform` (0.0 0.0 0.0)) "AlwaysSpawn" "MultiplyWithRoot" null self null))
        (set `self.SelectedAction_RightClick` _returnvalue_2)))
    (:`then_2`
      (`self.OnSelectedActionsChanged` (`self.SelectedAction_LeftClick`) (`self.SelectedAction_RightClick`)))))

(fn `UpdateHoveredTile`
  (bind _hoveredtile (`self.HoveredTile`))
  (bind _outindex (`/Game/Blueprints/Grid/BP_Grid.GetTileIndexUnderCursor` (`self.Grid`) 0))
  (if (!= _outindex _hoveredtile)
    (`/Game/Blueprints/Grid/BP_Grid.RemoveStateFromTile` (`self.Grid`) _hoveredtile "NewEnumerator1")
    (set `self.HoveredTile` _outindex)
    (`/Game/Blueprints/Grid/BP_Grid.AddStateToTile` (`self.Grid`) (`self.HoveredTile`) "NewEnumerator1")
    (`self.OnHoverTileChanged`)))

(fn `UserConstructionScript`)